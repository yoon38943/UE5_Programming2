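; BP_EX03_2 is an exercise actor that moves along world X or Y according to a current direction state.
; Tick switches on CurrentDir: T, G, F and H step the location by MoveVal times delta seconds, while Space holds it at the world origin.
; MoveVector sets CurrentDir and flags ChangeDir when the direction differs, though nothing here calls it or reads that flag.
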(event EventTick
  (params (DeltaSeconds :type Float%20%28single-precision%29))
  (bind _returnvalue (Transformation|GetActorLocation))
  (bind _returnvalue_2 (Transformation|GetActorLocation))
  (bind _returnvalue_3 (Transformation|GetActorLocation))
  (bind _returnvalue_4 (Transformation|GetActorLocation))
  (Variables|Default|SetDelta%20Seconds DeltaSeconds)
  (switch Utilities|FlowControl|Switch|SwitchonDirection (Variables|Default|GetCurrentDir)
    (:NewEnumerator0
      (Transformation|SetActorLocation (Math|Vector|MakeVector (+ (.x _returnvalue_4) (* (Variables|Default|GetDelta%20Seconds) (Variables|Default|GetMoveVal))) (.y _returnvalue_4) (.z _returnvalue_4)) false false))
    (:NewEnumerator2
      (Transformation|SetActorLocation (Math|Vector|MakeVector (+ (.x _returnvalue) (* (* (Variables|Default|GetDelta%20Seconds) (Variables|Default|GetMoveVal)) -1.0)) (.y _returnvalue) (.z _returnvalue)) false false))
    (:NewEnumerator3
      (Transformation|SetActorLocation (Math|Vector|MakeVector (.x _returnvalue_2) (+ (.y _returnvalue_2) (* (* (Variables|Default|GetDelta%20Seconds) (Variables|Default|GetMoveVal)) -1.0)) (.z _returnvalue_2)) false false))
    (:NewEnumerator4
      (Transformation|SetActorLocation (Math|Vector|MakeVector (.x _returnvalue_3) (+ (.y _returnvalue_3) (* (Variables|Default|GetDelta%20Seconds) (Variables|Default|GetMoveVal))) (.z _returnvalue_3)) false false))
    (:NewEnumerator5
      (Transformation|SetActorLocation "0, 0, 0" false false))))

(fn ConstructionScript)

(fn MoveVector
  (params (inDir :type Direction%20Enum :default "NewEnumerator0"))
  (if (Utilities|Enum|NotEqual(Enum) inDir (Variables|Default|GetCurrentDir))
    (Variables|Default|SetChangeDir true)
    (else
      (Variables|Default|SetChangeDir false)))
  (Variables|Default|SetCurrentDir inDir))