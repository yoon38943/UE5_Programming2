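; BP_Actor01 is an exercise actor that prints its own identity and transform on screen when play begins.
; BeginPlay prints the display name, then the location, rotation and scale of the actor transform, with scale in a custom color.
; All prints share a PrintDuration variable, and Korean comments note struct pin splitting and that GetDisplayName returns the Outliner label.
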(event EventBeginPlay
  (bind _self self)
  (bind _printduration (Variables|Default|GetPrintDuration))
  (bind _returnvalue (Transformation|GetActorTransform _self))
  (Development|PrintString (Utilities|GetDisplayName _self) true true "(R=0.000000,G=0.660000,B=1.000000,A=1.000000)" _printduration)
  (Development|PrintString (Utilities|String|ToString(Vector) (.location _returnvalue)) true true "(R=0.000000,G=0.660000,B=1.000000,A=1.000000)" _printduration)
  (Development|PrintString (Utilities|String|ToString(Rotator) (.rotation _returnvalue)) true true "(R=0.000000,G=0.660000,B=1.000000,A=1.000000)" _printduration)
  (Development|PrintString (Utilities|String|ToString(Vector) (.scale _returnvalue)) true true "(R=1.000000,G=0.057191,B=0.764297,A=1.000000)" _printduration))

(fn ConstructionScript)