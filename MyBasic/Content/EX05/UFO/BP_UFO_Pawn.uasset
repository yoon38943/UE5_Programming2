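; Player-controlled UFO pawn that flies, shoots projectiles and periodically spawns spheres ahead of itself.
; BeginPlay adds the UFO Enhanced Input mapping context, whose actions drive movement along the forward vector, controller yaw and pitch, and shooting with a fire sound.
; Tick accumulates delta time to spawn a BP_GC_Sphere far in front every two seconds, passing it the reversed forward vector via ToMe.
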(event Input|EnhancedActionEvents|EnhancedInputActionIA_MoveUFO
  (params (ActionValue :type Float%20%28double-precision%29) (ElapsedSeconds :type Float%20%28double-precision%29) (TriggeredSeconds :type Float%20%28double-precision%29) (InputAction :type Input%20Action%20Object%20Reference :default "/Game/EX05/UFO/Input/IA_MoveUFO.IA_MoveUFO"))
  (Utilities|IsValid (Pawn|GetController)
    (:Is%20Valid
      (Pawn|Input|AddMovementInput (Transformation|GetActorForwardVector) ActionValue false))))

(event Input|EnhancedActionEvents|EnhancedInputActionIA_LookUFO
  (params (ActionValue :type Vector%202D%20Structure) (ElapsedSeconds :type Float%20%28double-precision%29) (TriggeredSeconds :type Float%20%28double-precision%29) (InputAction :type Input%20Action%20Object%20Reference :default "/Game/EX05/UFO/Input/IA_LookUFO.IA_LookUFO"))
  (Pawn|Input|AddControllerYawInput (.x ActionValue))
  (Pawn|Input|AddControllerPitchInput (.y ActionValue)))

(event Input|EnhancedActionEvents|EnhancedInputActionIA_Shot
  (params (ActionValue :type Boolean) (ElapsedSeconds :type Float%20%28double-precision%29) (TriggeredSeconds :type Float%20%28double-precision%29) (InputAction :type Input%20Action%20Object%20Reference :default "/Game/EX05/UFO/Input/IA_Shot.IA_Shot"))
  (:Started
    (bind _returnvalue (Game|SpawnActorfromClass "/Game/EX05/UFO/BP_ProjectTile.BP_ProjectTile_C" (Math|Transform|MakeTransform (Transformation|GetActorLocation) (Transformation|GetActorRotation) "1.000000,1.000000,1.000000") "Undefined" "MultiplyWithRoot" 0 0))
    (Default|Launch _returnvalue)
    (Audio|PlaySoundatLocation "/Game/_Asset/Sound/FirstPersonTemplateWeaponFire02.FirstPersonTemplateWeaponFire02" (Transformation|GetActorLocation) "0, 0, 0" 1.0 1.0 0.0 0 0 0 0)))

(event EventBeginPlay
  (bind _as플레이어_컨트롤러 (Utilities|Casting|CastToPlayerController (Pawn|GetController)))
  (Input|AddMappingContext (PlayerController|LocalPlayerSubsystems|GetEnhancedInputLocalPlayerSubsystem _as플레이어_컨트롤러) "/Game/EX05/UFO/Input/IMC_UFO.IMC_UFO" 0 "(bIgnoreAllPressedKeysUntilRelease=True,bForceImmediately=False,bNotifyUserSettings=False)"))

(event EventTick
  (params (DeltaSeconds :type Float%20%28single-precision%29))
  (bind _returnvalue (Transformation|GetActorForwardVector))
  (bind _output_get (Variables|Default|SetDeltaTime (+ DeltaSeconds (Variables|Default|GetDeltaTime))))
  (if (>= _output_get 2.0)
    (Variables|Default|SetDeltaTime 0.0)
    (bind _returnvalue_2 (Game|SpawnActorfromClass "/Game/EX05/BP_GC_Sphere.BP_GC_Sphere_C" (Math|Transform|MakeTransform (+ (* _returnvalue 5e+03) (Transformation|GetActorLocation)) "0, 0, 0" "1.000000,1.000000,1.000000") "Undefined" "MultiplyWithRoot" 0 0))
    (Default|ToMe _returnvalue_2 (* _returnvalue -1.0))))

(fn ConstructionScript)