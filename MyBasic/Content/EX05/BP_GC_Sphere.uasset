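; BP_GC_Sphere is a sphere actor that spins until a projectile hits it, then disappears.
; Tick yaws it by RotateSpeed until the first BP_ProjectTile overlap sets the Overlap flag.
; That overlap stops the spin, plays a collapse sound and starts a timer that destroys the actor three seconds later.
; ToMe stores SphereVector, which only disconnected movement nodes read.
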(event OnComponentBeginOverlap(Sphere)
  (params (OverlappedComponent :type Primitive%20Component%20Object%20Reference) (OtherActor :type Actor%20Object%20Reference) (OtherComp :type Primitive%20Component%20Object%20Reference) (OtherBodyIndex :type Integer) (bFromSweep :type Boolean) (SweepResult :type Hit%20Result%20Structure%20%28by%20ref%29))
  (if (not (Variables|Default|GetOverlap))
    (Utilities|Casting|CastToBP_ProjectTile OtherActor)
    (Audio|PlaySound2D "/Game/_Asset/Sound/Collapse01.Collapse01" 1.0 1.0 0.0 0 0)
    (Variables|Default|SetOverlap true)
    (Utilities|Time|SetTimerbyEvent (delegate Custom|Destroy) 3.0)))

(event Custom|Destroy
  (Actor|DestroyActor))

(event EventBeginPlay)

(event EventTick
  (params (DeltaSeconds :type Float%20%28single-precision%29))
  (if (not (Variables|Default|GetOverlap))
    (Transformation|AddActorLocalRotation (Math|Rotator|MakeRotator 0.0 0.0 (* DeltaSeconds (Variables|Default|GetRotateSpeed))) false false)))

(fn ConstructionScript)

(fn ToMe
  (params (NewParam :type Vector))
  (Variables|Default|SetSphereVector NewParam))