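; BP_SolaSystem is an actor that models a simple solar system with Sun, Earth and Moon components.
; The construction script sets each body's world scale from the SunScale, EarthScale and MoonScale variables.
; Tick spins the AxisEarth pivot in local yaw at a constant, delta-time-scaled rate.
; A slower relative yaw rotation for AxisSun exists in the graph but is disconnected, so it never runs.
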(event EventBeginPlay)

(event Collision|EventActorBeginOverlap
  (params (OtherActor :type Actor%20Object%20Reference)))

(event EventTick
  (params (DeltaSeconds :type Float%20%28single-precision%29))
  (Transformation|AddLocalRotation (Variables|Default|GetAxisEarth) (Math|Rotator|MakeRotator 0.0 0.0 (* DeltaSeconds 5e+01)) false false))

(fn ConstructionScript
  (Transformation|SetWorldScale3D (Variables|Default|GetSun) (Variables|Default|GetSunScale))
  (Transformation|SetWorldScale3D (Variables|Default|GetEarth) (Variables|Default|GetEarthScale))
  (Transformation|SetWorldScale3D (Variables|Default|GetMoon) (Variables|Default|GetMoonScale)))